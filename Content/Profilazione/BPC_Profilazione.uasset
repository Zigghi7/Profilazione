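; Profilazione (profiling) component that opens the profiling menu when play begins.
; It finds BP_ProfilazioneController in the level and reads its base URL, contest name (NomeConcorso) and contest center (CentroConcorso).
; It passes these values into a new WBP_MenuProfilazione for the first player, adds the widget to the viewport and shows the mouse cursor.
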(event `self.ReceiveBeginPlay`
  (bind _returnvalue (`GameplayStatics.GetActorOfClass` "/Game/Profilazione/BP_ProfilazioneController.BP_ProfilazioneController_C"))
  (set `self.Url Filezilla` (`/Game/Profilazione/BP_ProfilazioneController.In Base Url` _returnvalue))
  (set `self.NomeConcorso` (`/Game/Profilazione/BP_ProfilazioneController.NomeConcorso` _returnvalue))
  (set `self.CentroConcorso` (`/Game/Profilazione/BP_ProfilazioneController.CentroConcorso` _returnvalue))
  (bind _returnvalue_2 (`|CreateWidget` "/Game/Profilazione/WBP_MenuProfilazione.WBP_MenuProfilazione_C" (`GameplayStatics.GetPlayerController` 0) (`self.Url Filezilla`) (`self.NomeConcorso`) (`self.CentroConcorso`)))
  (bind _output_get (set `self.WidgetMenuProfilazione` _returnvalue_2))
  (`UserWidget.AddToViewport` _output_get 0)
  (set `PlayerController.bShowMouseCursor` true (`GameplayStatics.GetPlayerController` 0)))